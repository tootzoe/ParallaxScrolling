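; BP_BgParallax1 is a scrolling parallax background actor driven by a five-layer material.
; On BeginPlay it creates a dynamic instance of M_Parallax1 on its static mesh.
; Each tick it advances an offset by ParallaxVelocity, wrapping it past 1.0.
; It feeds that offset to the material's per-layer X offset parameters, doubling it for each successive layer so they scroll at different speeds.
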(event EventBeginPlay
  (bind _returnvalue (Rendering|Material|CreateDynamicMaterialInstance (Variables|Debug|GetStaticMeshComponent) 0 "/Game/Texture/Bg/Parallax1/M_Parallax1.M_Parallax1" "None" :!class /Script/Engine.PrimitiveComponent))
  (Variables|Default|SetBgMat _returnvalue))

(event Collision|EventActorBeginOverlap
  (params (OtherActor :type Actor%20Object%20Reference)))

(event EventTick
  (params (DeltaSeconds :type Float%20%28single-precision%29))
  (|UpdParallaxOffset DeltaSeconds
    (:OutputPin
      (CallFunction|UpdParallaxScrolling (Variables|Default|GetParallaxOffset)))))

(fn ConstructionScript)

(fn UpdParallaxScrolling
  (params (XOffset :type Float%20%28single-precision%29))
  (bind _returnvalue (* XOffset 2.0))
  (bind _returnvalue_2 (* _returnvalue 2.0))
  (bind _returnvalue_3 (* _returnvalue_2 2.0))
  (Rendering|Material|SetScalarParameterValue (Variables|Default|GetBgMat) "XOffsetLayer0" XOffset :!class /Script/Engine.MaterialInstanceDynamic)
  (Rendering|Material|SetScalarParameterValue (Variables|Default|GetBgMat) "XOffsetLayer1" _returnvalue :!class /Script/Engine.MaterialInstanceDynamic)
  (Rendering|Material|SetScalarParameterValue (Variables|Default|GetBgMat) "XOffsetLayer2" _returnvalue_2 :!class /Script/Engine.MaterialInstanceDynamic)
  (Rendering|Material|SetScalarParameterValue (Variables|Default|GetBgMat) "XOffsetLayer3" _returnvalue_3 :!class /Script/Engine.MaterialInstanceDynamic)
  (Rendering|Material|SetScalarParameterValue (Variables|Default|GetBgMat) "XOffsetLayer4" (* _returnvalue_3 2.0) :!class /Script/Engine.MaterialInstanceDynamic))